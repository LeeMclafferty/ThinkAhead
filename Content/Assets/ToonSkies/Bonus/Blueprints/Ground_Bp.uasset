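; Ground actor from the ToonSkies bonus content that provides a configurable, noise-textured ground surface.
; The Construction Script creates a dynamic instance of GroundMaterial_M on the Ground component and feeds it noise size, noise strength and a color picked from GroundColorList by ColorNumber.
; It also pins the root to the world origin in X and Y, keeping only its height; there is no runtime logic.
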(event EventBeginPlay)

(event Collision|EventActorBeginOverlap
  (params (OtherActor :type Actor%20Object%20Reference)))

(event EventTick
  (params (DeltaSeconds :type Float%20%28single-precision%29)))

(fn ConstructionScript
  (bind _defaultsceneroot (Variables|Default|GetDefaultSceneRoot))
  (bind _returnvalue (Rendering|Material|CreateDynamicMaterialInstance (Variables|Default|GetGround) 0 "/Game/Assets/ToonSkies/Bonus/Materials/GroundMaterial_M.GroundMaterial_M" "None" :!class /Script/Engine.PrimitiveComponent))
  (Rendering|Material|SetScalarParameterValue _returnvalue "NoiseSize" (Variables|Default|GetNoiseSize) :!class /Script/Engine.MaterialInstanceDynamic)
  (Rendering|Material|SetScalarParameterValue _returnvalue "NoiseStrength" (Variables|Default|GetNoiseStrength) :!class /Script/Engine.MaterialInstanceDynamic)
  (Rendering|Material|SetVectorParameterValue _returnvalue "GroundColor" (Utilities|Array|Get(acopy) (Variables|Default|GetGroundColorList) (Variables|Default|GetColor%20Number)) :!class /Script/Engine.MaterialInstanceDynamic)
  (Transformation|SetWorldLocation _defaultsceneroot (Math|Vector|MakeVector 0.0 0.0 (.z (Transformation|GetWorldLocation _defaultsceneroot))) false false))