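; Toon sky dome actor that drives a dynamic material on a sky sphere for stylized clouds, stars, sun or moon, gradients and lighting.
; Construction script centers it at world origin, then pushes custom or preset settings into the material, with day/night preview.
; BeginPlay holds timeline logic animating planet, colors, stars and lighting through a day cycle, but its branch is hardwired false, so it never runs.
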(event EventBeginPlay
  (bind _dynamic (Variables|Texture|GetDynamic))
  (bind _day_night_cycle (Variables|Default|GetDay%20Night%20Cycle))
  (Utilities|DayCycleVariables)
  (if false
    (Utilities|FlowControl|Sequence
      (:then_0
        (bind (_direction _planetheights _skylerp _stars _lightingstrength) (Timeline|Day%20Night%20Cycle SetNewTime)
          (:Update
            (Rendering|Material|SetScalarParameterValue (Variables|Texture|GetDynamic) "PlanetY" _planetheights :!class /Script/Engine.MaterialInstanceDynamic)
            (if (Variables|Bools|GetLightingDnCycle)
              (Rendering|Material|SetScalarParameterValue (Variables|Texture|GetDynamic) "LightingStrength" (Math|Float|Lerp 0.0 (Variables|Floats|GetLightingStrength) _lightingstrength) :!class /Script/Engine.MaterialInstanceDynamic))
            (Components|Timeline|SetPlayRate _day_night_cycle (/ (Components|Timeline|GetTimelineLength _day_night_cycle) (Variables|DayNightCycle|GetDay%20Length)))
            (Rendering|Material|SetVectorParameterValue _dynamic "Overall Color" (Math|Color|Lerp(LinearColor) (Variables|DayNightCycle|GetDay%20Overall%20Color) (Variables|DayNightCycle|GetNight%20Overall%20Color) _skylerp) :!class /Script/Engine.MaterialInstanceDynamic)
            (Rendering|Material|SetScalarParameterValue _dynamic "StarsBrightness" (Math|Float|Lerp 0.0 (.Brightness (Utilities|Struct|BreakStars_S (.Stars (Utilities|Struct|BreakDefaults_S (.Defaults (Utilities|Struct|BreakCustomSetting_S (Variables|Default|GetCustomSetting))))))) _stars) :!class /Script/Engine.MaterialInstanceDynamic)
            (if (Math|Float|InRange(Float) (Components|Timeline|GetPlaybackPosition (Variables|Default|GetDay%20Night%20Cycle)) 0.2 0.8)
              (Utilities|FlowControl|DoOnce false
                (:Completed
                  (Rendering|Material|SetTextureParameterValue (Variables|Texture|GetDynamic) "PlanetT" (Variables|DayNightCycle|GetSun%20Style))
                  (Rendering|Material|SetVectorParameterValue (Variables|Texture|GetDynamic) "PlanetColor" (Variables|DayNightCycle|GetSun%20Color) :!class /Script/Engine.MaterialInstanceDynamic)))
              (else
                (Utilities|FlowControl|DoOnce false
                  (:Completed
                    (Rendering|Material|SetTextureParameterValue (Variables|Texture|GetDynamic) "PlanetT" (Variables|DayNightCycle|GetMoon%20Style))
                    (Rendering|Material|SetVectorParameterValue (Variables|Texture|GetDynamic) "PlanetColor" (Variables|DayNightCycle|GetMoon%20Color) :!class /Script/Engine.MaterialInstanceDynamic))))))
          (:NightPlanet
            (Rendering|Material|SetTextureParameterValue (Variables|Texture|GetDynamic) "PlanetT" (Variables|DayNightCycle|GetMoon%20Style))
            (Rendering|Material|SetVectorParameterValue (Variables|Texture|GetDynamic) "PlanetColor" (Variables|DayNightCycle|GetMoon%20Color) :!class /Script/Engine.MaterialInstanceDynamic))
          (:DayPlanet
            (Rendering|Material|SetTextureParameterValue (Variables|Texture|GetDynamic) "PlanetT" (Variables|DayNightCycle|GetSun%20Style))
            (Rendering|Material|SetVectorParameterValue (Variables|Texture|GetDynamic) "PlanetColor" (Variables|DayNightCycle|GetSun%20Color) :!class /Script/Engine.MaterialInstanceDynamic))))
      (:then_1
        (Timeline|Day%20Night%20Cycle Play)))))

(fn ConstructionScript
  ;[1 1 1] Center the Sky Sphere
  (Transformation|SetWorldLocation (Variables|Default|GetDefaultSceneRoot) "0, 0, 0" false false)
  ;[1 1 1] Apply ToonSky
  (switch Utilities|FlowControl|Switch|SwitchonSkyType_E (Variables|Default|GetType)
    (:NewEnumerator0
      (CallFunction|PresetFunction))
    (:NewEnumerator1
      _))
  ;[1 1 1] Set Dynamic Sky Dynamic Material
  (bind _returnvalue (Rendering|Material|CreateDynamicMaterialInstance (Variables|Default|GetSkySphereMesh) 0 "/Game/Assets/ToonSkies/Materials/TypeB_M_Inst.TypeB_M_Inst" "None" :!class /Script/Engine.PrimitiveComponent))
  (Variables|Texture|SetDynamic _returnvalue)
  ;[1 1 1] Apply Sky Material Setting
  (CallFunction|SetColors)
  (CallFunction|GetColors)
  (CallFunction|SetDefaults)
  (CallFunction|Clouds)
  (CallFunction|Stars)
  (Utilities|PlanetSetting)
  (CallFunction|Styles))

(fn SetColors
  (bind _customsetting (Variables|Default|GetCustomSetting))
  (bind (_defaults _colors _styles _lighting) (Utilities|Struct|BreakCustomSetting_S _customsetting))
  (bind (_firstcloudcolor _secondcloudcolor _starscolor _horizoncolor _horizonfalloff _overallcolor _planetcolor _environmentcolor _environmentcolorthreshold _skygradient1 _skygradient2 _gradientstrength _skydiffuse) (Utilities|Struct|BreakColors_S _colors))
  (bind (_lightingstrength _lightingcolor _daynightcycle) (Utilities|Struct|BreakLighting_S _lighting))
  (|ApplyColors _firstcloudcolor _secondcloudcolor _starscolor _horizoncolor _horizonfalloff _overallcolor _planetcolor _environmentcolor _environmentcolorthreshold _skygradient1 _skygradient2 _gradientstrength _skydiffuse _lightingstrength _lightingcolor _daynightcycle)
  (return))

(fn GetColors
  (bind _day___night_cycle (Variables|Default|GetDay%20&%20Night%20Cycle))
  (bind (_daynightcycle _preview _daylength _timeofday _sunstyle _moonstyle _dayoverallcolor _nightoverallcolor) (Utilities|Struct|BreakDayCycle_S _day___night_cycle))
  ;[1 1 1] Is DayNight Cycle Applied?
  (if _daynightcycle
    ;[1 1 1] Preview Day / Night
    (switch Utilities|FlowControl|Switch|SwitchonDayCyclePreview_E _preview
      (:NewEnumerator0
        (Rendering|Material|SetVectorParameterValue (Variables|Texture|GetDynamic) "Overall Color" _dayoverallcolor :!class /Script/Engine.MaterialInstanceDynamic))
      (:NewEnumerator1
        (Rendering|Material|SetVectorParameterValue (Variables|Texture|GetDynamic) "Overall Color" _nightoverallcolor :!class /Script/Engine.MaterialInstanceDynamic)))
    (else
      (Rendering|Material|SetVectorParameterValue (Variables|Texture|GetDynamic) "Overall Color" (Variables|Colors|GetOverallColor) :!class /Script/Engine.MaterialInstanceDynamic)))
  ;[1 1 1] Change Material Parameters
  (Rendering|Material|SetVectorParameterValue (Variables|Texture|GetDynamic) "FirstColor" (Variables|Colors|GetFirstCloudColor) :!class /Script/Engine.MaterialInstanceDynamic)
  (Rendering|Material|SetVectorParameterValue (Variables|Texture|GetDynamic) "SecondColor" (Variables|Colors|GetSecondCloudColor) :!class /Script/Engine.MaterialInstanceDynamic)
  (Rendering|Material|SetVectorParameterValue (Variables|Texture|GetDynamic) "StarsColor" (Variables|Colors|GetStarsColor) :!class /Script/Engine.MaterialInstanceDynamic)
  (Rendering|Material|SetVectorParameterValue (Variables|Texture|GetDynamic) "EnvColor" (Variables|Colors|GetEnvColor) :!class /Script/Engine.MaterialInstanceDynamic)
  (Rendering|Material|SetVectorParameterValue (Variables|Texture|GetDynamic) "Grad1" (Variables|Colors|GetSkyG1) :!class /Script/Engine.MaterialInstanceDynamic)
  (Rendering|Material|SetVectorParameterValue (Variables|Texture|GetDynamic) "Grad2" (Variables|Colors|GetSkyG2) :!class /Script/Engine.MaterialInstanceDynamic)
  (Rendering|Material|SetVectorParameterValue (Variables|Texture|GetDynamic) "GradDiff" (Variables|Colors|GetSkyDiffuse) :!class /Script/Engine.MaterialInstanceDynamic)
  (Rendering|Material|SetScalarParameterValue (Variables|Texture|GetDynamic) "GradStrength" (Variables|Floats|GetGradStrength) :!class /Script/Engine.MaterialInstanceDynamic)
  (Rendering|Material|SetScalarParameterValue (Variables|Texture|GetDynamic) "Falloff" (Variables|Floats|GetHorizonFallOff) :!class /Script/Engine.MaterialInstanceDynamic)
  (Rendering|Material|SetVectorParameterValue (Variables|Texture|GetDynamic) "HorizonColor" (Variables|Colors|GetHorizonColor) :!class /Script/Engine.MaterialInstanceDynamic)
  (Rendering|Material|SetVectorParameterValue (Variables|Texture|GetDynamic) "LightingColor" (Variables|Colors|GetLightingColor) :!class /Script/Engine.MaterialInstanceDynamic)
  (Rendering|Material|SetScalarParameterValue (Variables|Texture|GetDynamic) "LightingStrength" (Variables|Floats|GetLightingStrength) :!class /Script/Engine.MaterialInstanceDynamic)
  (Rendering|Material|SetScalarParameterValue (Variables|Texture|GetDynamic) "ColorThreshold" (Variables|Floats|GetEnvColorThreshold) :!class /Script/Engine.MaterialInstanceDynamic)
  (return))

(fn SetDefaults
  (bind _customsetting (Variables|Default|GetCustomSetting))
  (bind _day___night_cycle (Variables|Default|GetDay%20&%20Night%20Cycle))
  (bind _day___night_cycle_2 (Variables|Default|GetDay%20&%20Night%20Cycle))
  (bind _defaults (Utilities|Struct|BreakCustomSetting_S _customsetting))
  (bind (_daynightcycle _preview _daylength _timeofday _sunstyle _moonstyle _dayoverallcolor _nightoverallcolor _suncolor _mooncolor) (Utilities|Struct|BreakDayCycle_S _day___night_cycle_2))
  (bind (_firstcloud _secondcloud _stars) (Utilities|Struct|BreakDefaults_S _defaults))
  (bind (_addstars _animated _brightness _density) (Utilities|Struct|BreakStars_S _stars))
  (bind _returnvalue (Math|Float|Clamp(Float) _density 2.0 3.0))
  ;[1 1 1] Clouds Defaults
  (Utilities|FirstCloudSetting _firstcloud)
  (Utilities|SecondCloudSetting _secondcloud)
  ;[1 1 1] Planet Setting
  (Utilities|PlanetSetting)
  ;[1 1 1] Stars Defaults
  (Variables|Bools|SetAddStars _addstars)
  (Variables|Bools|SetAnimateStars _animated)
  (Variables|Floats|SetStarsBrightness _brightness)
  (Utilities|Struct|SetmembersinStars_S (.Stars (Utilities|Struct|BreakDefaults_S (.Defaults (Utilities|Struct|BreakCustomSetting_S (Variables|Default|GetCustomSetting))))) _returnvalue)
  (Variables|Floats|SetStarsDensity _returnvalue)
  ;[1 1 1] Time Of Day 24 Hours Format
  (Utilities|Struct|SetmembersinDayCycle_S _day___night_cycle (Math|Float|Clamp(Float) (.TimeOfDay (Utilities|Struct|BreakDayCycle_S _day___night_cycle)) 0.0 24.0))
  ;[1 1 1] DayNight Cycle
  (if _daynightcycle
    (switch Utilities|FlowControl|Switch|SwitchonDayCyclePreview_E _preview
      (:NewEnumerator0
        (Rendering|Material|SetVectorParameterValue (Variables|Texture|GetDynamic) "PlanetColor" _suncolor :!class /Script/Engine.MaterialInstanceDynamic))
      (:NewEnumerator1
        (Rendering|Material|SetVectorParameterValue (Variables|Texture|GetDynamic) "PlanetColor" _mooncolor :!class /Script/Engine.MaterialInstanceDynamic)))
    (else
      (Rendering|Material|SetVectorParameterValue (Variables|Texture|GetDynamic) "PlanetColor" (Variables|Colors|GetPlanetColor) :!class /Script/Engine.MaterialInstanceDynamic)))
  (return))

(fn Clouds
  ;[1 1 1] First Clouds
  (Rendering|Material|SetScalarParameterValue (Variables|Texture|GetDynamic) "FirstMoveY" (Variables|Floats|GetFirstHeight) :!class /Script/Engine.MaterialInstanceDynamic)
  (Rendering|Material|SetScalarParameterValue (Variables|Texture|GetDynamic) "SpeedFirst" (* (Variables|Floats|GetSpeedFirst) 0.01) :!class /Script/Engine.MaterialInstanceDynamic)
  (Rendering|Material|SetScalarParameterValue (Variables|Texture|GetDynamic) "FirstOpacity" (Variables|Floats|GetFirstOpacity) :!class /Script/Engine.MaterialInstanceDynamic)
  ;[1 1 1] Second Clouds
  (Rendering|Material|SetScalarParameterValue (Variables|Texture|GetDynamic) "SecondMoveY" (Variables|Floats|GetSecondHeight) :!class /Script/Engine.MaterialInstanceDynamic)
  (Rendering|Material|SetScalarParameterValue (Variables|Texture|GetDynamic) "SpeedSecond" (* (Variables|Floats|GetSpeedSecond) 0.01) :!class /Script/Engine.MaterialInstanceDynamic)
  (Rendering|Material|SetScalarParameterValue (Variables|Texture|GetDynamic) "SecondOpacity" (Variables|Floats|GetSecondOpacity) :!class /Script/Engine.MaterialInstanceDynamic)
  (return))

(fn Stars
  ;[1 1 1] Stars Setting
  (if (Variables|Bools|GetAddStars)
    (Rendering|Material|SetScalarParameterValue (Variables|Texture|GetDynamic) "StarsBrightness" (Variables|Floats|GetStarsBrightness) :!class /Script/Engine.MaterialInstanceDynamic)
    (else
      (Rendering|Material|SetScalarParameterValue (Variables|Texture|GetDynamic) "StarsBrightness" 0.0 :!class /Script/Engine.MaterialInstanceDynamic)))
  (Rendering|Material|SetScalarParameterValue (Variables|Texture|GetDynamic) "StarsScale" (Variables|Floats|GetStarsDensity) :!class /Script/Engine.MaterialInstanceDynamic)
  ;[1 1 1] Stars Animation
  (if (Variables|Bools|GetAnimateStars)
    (Rendering|Material|SetScalarParameterValue (Variables|Texture|GetDynamic) "Animated" 1.0 :!class /Script/Engine.MaterialInstanceDynamic)
    (else
      (Rendering|Material|SetScalarParameterValue (Variables|Texture|GetDynamic) "Animated" 0.0 :!class /Script/Engine.MaterialInstanceDynamic)))
  (return))

(fn Styles
  (bind _customsetting (Variables|Default|GetCustomSetting))
  (bind _day___night_cycle (Variables|Default|GetDay%20&%20Night%20Cycle))
  (bind _styles (Utilities|Struct|BreakCustomSetting_S _customsetting))
  (bind (_daynightcycle _preview _daylength _timeofday _sunstyle _moonstyle) (Utilities|Struct|BreakDayCycle_S _day___night_cycle))
  (bind (_firstcloud _secondcloud _stars _planet _environment) (Utilities|Struct|BreakStyles_S _styles))
  ;[1 1 1] Set Textures
  (Variables|Texture|SetFirstCloud_T _firstcloud)
  (Variables|Texture|SetSecondClouds_T _secondcloud)
  (Variables|Texture|SetStars_T _stars)
  (Variables|Texture|SetPlanet_T _planet)
  (Variables|Texture|SetEnvironment_T _environment)
  ;[1 1 1] Get Textures
  (Rendering|Material|SetTextureParameterValue (Variables|Texture|GetDynamic) "FirstCloud" (Variables|Texture|GetFirstCloud_T))
  (Rendering|Material|SetTextureParameterValue (Variables|Texture|GetDynamic) "SecondCloud" (Variables|Texture|GetSecondClouds_T))
  (Rendering|Material|SetTextureParameterValue (Variables|Texture|GetDynamic) "StarsT" (Variables|Texture|GetStars_T))
  (Rendering|Material|SetTextureParameterValue (Variables|Texture|GetDynamic) "EnvT" (Variables|Texture|GetEnvironment_T))
  (if _daynightcycle
    (switch Utilities|FlowControl|Switch|SwitchonDayCyclePreview_E _preview
      (:NewEnumerator0
        (Rendering|Material|SetTextureParameterValue (Variables|Texture|GetDynamic) "PlanetT" _sunstyle))
      (:NewEnumerator1
        (Rendering|Material|SetTextureParameterValue (Variables|Texture|GetDynamic) "PlanetT" _moonstyle)))
    (else
      (Rendering|Material|SetTextureParameterValue (Variables|Texture|GetDynamic) "PlanetT" (Variables|Texture|GetPlanet_T))))
  (return))

(fn PresetFunction
  (switch Utilities|FlowControl|Switch|SwitchonPresetsEnum_E (Utilities|Struct|BreakPresetsEnums_S (Variables|Default|GetPresets))
    (:NewEnumerator21
      (|Index :!label _label))
    (:NewEnumerator22
      (goto _label 1))
    (:NewEnumerator23
      (goto _label 2))
    (:NewEnumerator24
      (goto _label 3))
    (:NewEnumerator25
      (goto _label 4))))

(fn LightingFunction)