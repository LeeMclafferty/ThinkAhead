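; BP_TestGrid is a grid actor that draws a tile grid of configurable rows, columns and tile size as procedural geometry.
; The construction script loops over rows and columns, and CreateLine appends each line as a thick two-triangle quad into shared arrays for one mesh section.
; Lines use a dynamic material instance with color and opacity.
; A selection material is created but unused, and the tile lookup, validation and selection functions are stubs.
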(event EventBeginPlay)

(event Collision|EventActorBeginOverlap
  (params (OtherActor :type Actor%20Object%20Reference)))

(event EventTick
  (params (DeltaSeconds :type Float%20%28single-precision%29)))

(fn ConstructionScript
  (bind _newparam (CallFunction|CreateMaterialInstance (Variables|Generation|GetLineColor) (Variables|Generation|GetLineOpacity)))
  (LocalVariables|SetLinesMaterialInstance _newparam)
  (bind _newparam_2 (CallFunction|CreateMaterialInstance (Variables|Generation|GetSelectionColor) (Variables|Generation|GetSelectionOpacity)))
  (LocalVariables|SetSelectionMaterialInstance _newparam_2)
  (Utilities|FlowControl|Sequence
    (:then_0
      ;[1 1 1] Create Horizontal Lines Geometry
      (for _index (range 0 (Variables|Generation|GetNumColumns))
        (LocalVariables|SetLineStart (* _index (Variables|Generation|GetTileSize)))
        (LocalVariables|SetLineEnd (CallFunction|GridWidth))
        (CallFunction|CreateLine (Math|Vector|MakeVector (LocalVariables|GetLineStart) 0.0 0.0) (Math|Vector|MakeVector (LocalVariables|GetLineStart) (LocalVariables|GetLineEnd) 0.0) (Variables|Generation|GetLineThickness) (LocalVariables|GetLineVerticies) (LocalVariables|GetLineTriganles))))
    (:then_1
      ;[1 1 1] Create Vertical Lines Geometry
      (for _index_2 (range 0 (Variables|Generation|GetNumRows))
        (LocalVariables|SetLineStart (* _index_2 (Variables|Generation|GetTileSize)))
        (LocalVariables|SetLineEnd (CallFunction|GridHeight))
        (CallFunction|CreateLine (Math|Vector|MakeVector 0.0 (LocalVariables|GetLineStart) 0.0) (Math|Vector|MakeVector (LocalVariables|GetLineEnd) (LocalVariables|GetLineStart) 0.0) (Variables|Generation|GetLineThickness) (LocalVariables|GetLineVerticies) (LocalVariables|GetLineTriganles))))
    (:then_2
      ;[1 1 1] Create mesh with the lines
      (Class|ProceduralMeshComponent|CreateMeshSectionLinearColor (Variables|Default|GetProceduralMesh) 0 (LocalVariables|GetLineVerticies) (LocalVariables|GetLineTriganles) 0 0 0 0 0 0 0 false false)
      (Rendering|Material|SetMaterial (Variables|Default|GetProceduralMesh) 0 (LocalVariables|GetLinesMaterialInstance)))))

(fn CreateLine
  (params (Start :type Vector) (End :type Vector) (Thickness :type Float%20%28double-precision%29) (Verticies :type Array%20of%20Vectors) (Triangles :type Array%20of%20Integers))
  (bind _returnvalue (Utilities|Array|Length Verticies))
  (Utilities|FlowControl|Sequence
    (:then_0
      (LocalVariables|SetHalfThickness (/ Thickness 2.0))
      (LocalVariables|SetThicknessDirection (Math|Vector|CrossProduct (Math|Vector|Normalize (- End Start)) "0.000000,0.000000,1.000000")))
    (:then_1
      (Utilities|Array|AppendArray Triangles (Utilities|Array|MakeArray (+ 2 _returnvalue) (+ 1 _returnvalue) (+ 0 _returnvalue) (+ 2 _returnvalue) (+ 3 _returnvalue) (+ 1 _returnvalue)))
      (Utilities|Array|AppendArray Verticies (Utilities|Array|MakeArray (+ Start (* (LocalVariables|GetThicknessDirection) (LocalVariables|GetHalfThickness))) (+ End (* (LocalVariables|GetThicknessDirection) (LocalVariables|GetHalfThickness))) (- Start (* (LocalVariables|GetThicknessDirection) (LocalVariables|GetHalfThickness))) (- End (* (LocalVariables|GetThicknessDirection) (LocalVariables|GetHalfThickness))))))))

(fn GridWidth
  (return (* (Variables|Generation|GetNumColumns) (Variables|Generation|GetTileSize))))

(fn GridHeight
  (return (* (Variables|Generation|GetNumRows) (Variables|Generation|GetTileSize))))

(fn CreateMaterialInstance
  (params (Color :type Linear%20Color%20Structure) (Opacity :type Float%20%28double-precision%29))
  (bind _returnvalue (Rendering|Material|CreateDynamicMaterialInstance "/Game/Materials/Instances/M_Grid_Inst.M_Grid_Inst" "None" "None" :!class /Script/Engine.KismetMaterialLibrary))
  (Rendering|Material|SetVectorParameterValue _returnvalue "Color" Color :!class /Script/Engine.MaterialInstanceDynamic)
  (Rendering|Material|SetScalarParameterValue _returnvalue "Opacity" Opacity :!class /Script/Engine.MaterialInstanceDynamic)
  (return _returnvalue))

(fn LocationtoTile
  (params (Location :type Vector))
  (return 0 0 0))

(fn TiletoGridLocation
  (params (Row :type Integer) (Column :type Integer) (Center :type Boolean))
  (return false ""))

(fn SetSelectedTile
  (params (Row :type Integer) (Column :type Integer)))